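; GA_MeleeAttack is an enemy gameplay ability that turns the avatar toward its combat target and plays a random tagged attack montage.
; When the montage's gameplay event fires, it finds live players near that montage's combat socket and damages any non-friends.
; Hits spawn each victim's blood effect, plus one impact sound per strike.
; The ability ends when the montage finishes or is interrupted, or immediately if no montages exist.
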(event Ability|EventActivateAbility
  (bind _returnvalue (Ability|GetAvatarActorfromActorInfo))
  (bind _returnvalue_2 (Ability|GetAvatarActorfromActorInfo))
  (Variables|Default|SetHasHitTarget false)
  (bind _returnvalue_3 (Class|EnemyInterface|GetCombatTarget(Message) _returnvalue))
  (Class|CombatInterface|UpdateFacingTarget(Message) _returnvalue (Transformation|GetActorLocation _returnvalue_3))
  (bind _returnvalue_4 (Class|CombatInterface|GetAttackMontages(Message) _returnvalue))
  (if (Utilities|Array|IsNotEmpty _returnvalue_4)
    (Variables|Default|SetTaggedMontage (.OutItem (Utilities|Array|Random _returnvalue_4)))
    (|PlayMontageandWaitProxy "None" (.Montage (Utilities|Struct|BreakTaggedMontage (Variables|Default|GetTaggedMontage))) 1.0 "None" true 1.0 0.0 false
      (:then
        (Ability|Tasks|WaitGameplayEvent (.MontageTag (Utilities|Struct|BreakTaggedMontage (Variables|Default|GetTaggedMontage))) 0
          (:EventReceived
            (bind _returnvalue_5 (Class|CombatInterface|GetCombatSocketLocation(Message) _returnvalue_2 (.MontageTag (Utilities|Struct|BreakTaggedMontage (Variables|Default|GetTaggedMontage)))))
            (Variables|Default|SetCombatSocketLocation _returnvalue_5)
            (bind _outoverlappingactors (Class|MyAbilitySystemLibrary|GetLivePlayersWithinRadius (Utilities|Array|MakeArray _returnvalue_2) 45.0 (Variables|Default|GetCombatSocketLocation)))
            (for _array_element _outoverlappingactors
              (if (not (Class|MyAbilitySystemLibrary|IsFriend _array_element (Ability|GetAvatarActorfromActorInfo)))
                (Class|DamageGameplayAbility|CauseDamage _array_element)
                (Variables|Default|SetHasHitTarget true)
                (bind _ascombat_interface (Utilities|Casting|CastToCombatInterface _array_element))
                (bind _returnvalue_6 (Class|CombatInterface|GetBloodEffect _ascombat_interface))
                (Niagara|SpawnSystematLocation _returnvalue_6 (Variables|Default|GetCombatSocketLocation))))
            (if (Variables|Default|GetHasHitTarget)
              (Audio|PlaySoundatLocation (.ImpactSound (Utilities|Struct|BreakTaggedMontage (Variables|Default|GetTaggedMontage))) (Variables|Default|GetCombatSocketLocation) "0, 0, 0" 1.0 1.0 0.0 0 0 0 0)))))
      (:OnCompleted
        (Ability|EndAbility :!label _label))
      (:OnInterrupted
        (goto _label))
      (:OnCancelled
        (goto _label)))
    (else
      (Ability|EndAbility))))