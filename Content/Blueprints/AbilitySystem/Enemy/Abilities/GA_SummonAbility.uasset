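; Enemy gameplay ability for summoning, which so far only visualizes spawn points and does not spawn any actors.
; On activation it fetches positions from GetSpawnLocations, stores them and shuffles their order.
; A Delay-driven loop then steps through them with an index, drawing a brief debug sphere at each in staggered succession.
; The graph neither resets the index nor ends the ability.
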(event Ability|EventActivateAbility
  (bind _returnvalue (Class|SummonAbility|GetSpawnLocations))
  (bind _output_get (Variables|Default|SetSpawnLocations _returnvalue))
  (Utilities|Array|Shuffle _output_get)
  (if (< (Variables|Default|GetSpawnLocationIndex) (Utilities|Array|Length (Variables|Default|GetSpawnLocations))) :!label _label
    (Rendering|Debug|DrawDebugSphere (Utilities|Array|Get(acopy) (Variables|Default|GetSpawnLocations) (Variables|Default|GetSpawnLocationIndex)) 25.0 12 "(R=0.993406,G=0.960827,B=1.000000,A=1.000000)" 1.0)
    (Math|Integer|IncrementInt (Variables|Default|GetSpawnLocationIndex)
      (:%20%20
        (Utilities|FlowControl|Delay 0.2)
        (goto _label)))))