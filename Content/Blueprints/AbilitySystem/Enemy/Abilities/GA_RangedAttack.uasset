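; Enemy gameplay ability that performs a ranged attack by firing a projectile at the avatar's combat target.
; On activation it updates the avatar's facing toward the target and plays a random tagged attack montage, ending immediately if none exist.
; The montage's gameplay event triggers a projectile spawn from its socket tag, aimed at the target's location re-read at that moment.
; The ability ends when the montage completes, is interrupted or is cancelled.
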(event Ability|EventActivateAbility
  (bind _returnvalue (Ability|GetAvatarActorfromActorInfo))
  (bind _returnvalue_2 (Class|EnemyInterface|GetCombatTarget(Message) _returnvalue))
  (Class|CombatInterface|UpdateFacingTarget(Message) _returnvalue (Transformation|GetActorLocation _returnvalue_2))
  (bind _returnvalue_3 (Class|CombatInterface|GetAttackMontages(Message) (Ability|GetAvatarActorfromActorInfo)))
  (if (Utilities|Array|IsNotEmpty _returnvalue_3)
    (bind _output_get (Variables|Default|SetTaggedMontage (.OutItem (Utilities|Array|Random _returnvalue_3))))
    (|PlayMontageandWaitProxy "None" (.Montage (Utilities|Struct|BreakTaggedMontage _output_get)) 1.0 "None" false 1.0 0.0 false
      (:then
        (Ability|Tasks|WaitGameplayEvent (.MontageTag (Utilities|Struct|BreakTaggedMontage _output_get)) 0 true
          (:EventReceived
            (bind _returnvalue_4 (Class|EnemyInterface|GetCombatTarget(Message) (Ability|GetAvatarActorfromActorInfo)))
            (Class|ProjectileSpellBase|SpawnProjectile (Transformation|GetActorLocation _returnvalue_4) (.SocketTag (Utilities|Struct|BreakTaggedMontage (Variables|Default|GetTaggedMontage))) false 0.0))))
      (:OnCompleted
        (Ability|EndAbility :!label _label))
      (:OnInterrupted
        (goto _label))
      (:OnCancelled
        (goto _label)))
    (else
      (Ability|EndAbility))))